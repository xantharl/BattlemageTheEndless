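; GA_WallRun is the gameplay ability that drives wall running for the Battlemage character.
; On activation it asks the character's BMage movement component to start the WallRun movement ability and binds to that ability's end event.
; When the movement ability reports it is done, the gameplay ability ends itself.
; If cancelled early, it tells the movement component to end WallRun instead.
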(event Custom|OnMovementAbilityEnd_Event
  (params (MovementAbility :type Movement%20Ability%20Object%20Reference))
  ;[1 1 1 1 14] The custom MovementAbility Impl Fires this event when it decides the ability is done
  (Ability|EndAbility))

(event Ability|EventActivateAbility
  (bind _asbattlemage_the_endless_character (Utilities|Casting|CastToBattlemageTheEndlessCharacter (Ability|GetOwningActorfromActorInfo)))
  (bind _returnvalue (Class|BattlemagetheEndlessCharacter|GetBMageMovementComponent _asbattlemage_the_endless_character))
  (bind _returnvalue_2 (Class|BMageCharacterMovementComponent|TryStartAbility _returnvalue "WallRun"))
  ;[1 1 1 1 14] The custom MovementAbility Impl Fires this event when it decides the ability is done
  (bind _output_get (Variables|Default|SetMovementAbility _returnvalue_2))
  (EventDispatchers|AssignOnMovementAbilityEnd _output_get (delegate Custom|OnMovementAbilityEnd_Event)))

(event Ability|EventOnEndAbility
  (params (bWasCancelled :type Boolean))
  (if bWasCancelled
    (bind _asbattlemage_the_endless_character (Utilities|Casting|CastToBattlemageTheEndlessCharacter (Ability|GetOwningActorfromActorInfo)))
    (bind _returnvalue (Class|BattlemagetheEndlessCharacter|GetBMageMovementComponent _asbattlemage_the_endless_character))
    (Class|BMageCharacterMovementComponent|TryEndAbility _returnvalue "WallRun")))