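; GA_Slide is the gameplay ability for the Battlemage character's slide movement.
; On activation it plays an attached sliding sound and starts the Slide ability on the BMage movement component, then binds to that movement ability's end and transition-out events.
; The movement ability decides when the slide finishes, which ends the gameplay ability; both events stop and destroy the sound.
; A cancelled end tells the movement component to end the slide.
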(event Custom|OnMovementAbilityShouldTransitionOut_Event
  (params (MovementAbility :type Movement%20Ability%20Object%20Reference))
  (bind _slide_sound (Variables|Default|GetSlide%20Sound))
  (Audio|Components|Audio|Stop _slide_sound)
  (Components|DestroyComponent _slide_sound))

(event Custom|OnMovementAbilityEnd_Event
  (params (MovementAbility :type Movement%20Ability%20Object%20Reference))
  (bind _slide_sound (Variables|Default|GetSlide%20Sound))
  ;[1 1 1 1 14] The custom MovementAbility Impl Fires this event when it decides the ability is done
  (Ability|EndAbility)
  (Utilities|IsValid _slide_sound
    (:Is%20Valid
      (Audio|Components|Audio|Stop _slide_sound)
      (Components|DestroyComponent _slide_sound))))

(event Ability|EventActivateAbility
  (bind _returnvalue (Ability|GetOwningActorfromActorInfo))
  (bind _returnvalue_2 (Audio|SpawnSoundAttached "/Game/Sounds/Sliding.Sliding" (Variables|/Script/Engine.Actor|GetRootComponent _returnvalue) "None" "0, 0, 0" "0, 0, 0" "KeepRelativeOffset" false 1.0 1.0 0.0 "/Game/Characters/SoundAttenuation_Default.SoundAttenuation_Default" 0))
  (Variables|Default|SetSlide%20Sound _returnvalue_2)
  (bind _asbattlemage_the_endless_character (Utilities|Casting|CastToBattlemageTheEndlessCharacter _returnvalue))
  (bind _returnvalue_3 (Class|BattlemagetheEndlessCharacter|GetBMageMovementComponent _asbattlemage_the_endless_character))
  (bind _returnvalue_4 (Class|BMageCharacterMovementComponent|TryStartAbility _returnvalue_3 "Slide"))
  (bind _output_get (Variables|Default|SetMovementAbility _returnvalue_4))
  (Utilities|FlowControl|Sequence
    (:then_0
      ;[1 1 1 1 14] The custom MovementAbility Impl Fires this event when it decides the ability is done
      (EventDispatchers|AssignOnMovementAbilityEnd _output_get (delegate Custom|OnMovementAbilityEnd_Event)))
    (:then_1
      (EventDispatchers|AssignOnMovementAbilityShouldTransitionOut _output_get (delegate Custom|OnMovementAbilityShouldTransitionOut_Event)))))

(event Ability|EventOnEndAbility
  (params (bWasCancelled :type Boolean))
  (if bWasCancelled
    (bind _asbattlemage_the_endless_character (Utilities|Casting|CastToBattlemageTheEndlessCharacter (Ability|GetOwningActorfromActorInfo)))
    (bind _returnvalue (Class|BattlemagetheEndlessCharacter|GetBMageMovementComponent _asbattlemage_the_endless_character))
    (Class|BMageCharacterMovementComponent|TryEndAbility _returnvalue "Slide")))