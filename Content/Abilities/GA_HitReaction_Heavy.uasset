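; Gameplay Ability for the heavy hit reaction, triggered on AnimTraceHit from Character_AIBase and noted as cancelling both light and heavy attacks.
; Activation is allowed only when the owner's poise is broken, and fails if that check is unsuccessful.
; It starts the AM_OnHit montage through StartHitReaction, delays for the returned time, then ends the hit reaction and the ability.
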(event Ability|EventActivateAbility
  (bind _returnvalue (Ability|GetOwningActorfromActorInfo))
  ;[0.15 0.15 0.15 0.5 14] Heavy Hit reaction cancels light and heavy attacks, which light only cancels light
  (bind _stunduration (CallFunction|StartHitReaction _returnvalue "/Game/Animations/Skeleton/Sword_Shield/AM_OnHit.AM_OnHit" (Variables|Default|GetPlayRate)))
  (Utilities|FlowControl|Delay _stunduration)
  (CallFunction|EndHitReaction _returnvalue)
  (Ability|EndAbility))

(fn K2CanActivateAbility
  (params (ActorInfo :type Gameplay%20Ability%20Actor%20Info%20Structure) (Handle :type Gameplay%20Ability%20Spec%20Handle%20Structure))
  (bind (_isbroken _success) (CallFunction|IsPoiseBroken (.abilitysystemcomponent ActorInfo)))
  (if _success
    (return "" _isbroken)
    (else
      (return "" false))))