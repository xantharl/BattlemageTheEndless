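; Gameplay ability that plays a hit reaction montage on the owning Character and flags it as stunned.
; Only when the character is player-controlled, it sets IsStunned on the AI controller's blackboard and plays AM_OnHit.
; It waits out the montage, ends the ability, then clears the flag; other characters never reach EndAbility.
; Movement and brain-logic stop/start nodes are present but never run.
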(event Ability|EventActivateAbility
  (bind _ascharacter (Utilities|Casting|CastToCharacter (Ability|GetOwningActorfromActorInfo)))
  (bind _output_get (Variables|Default|SetIsPlayerControlled (Pawn|IsPlayerControlled _ascharacter)))
  (if _output_get
    (AI|Components|Blackboard|SetValueasBool (AI|GetBlackboard (AI|GetAIController _ascharacter)) (Utilities|Name|MakeLiteralName "IsStunned") true)
    (bind _returnvalue (Animation|PlayAnimMontage _ascharacter "/Game/Animations/Skeleton/Sword_Shield/AM_OnHit.AM_OnHit" 1.0 "None"))
    (if (> _returnvalue 0.0)
      (Utilities|FlowControl|Delay _returnvalue))
    (Ability|EndAbility)
    (if (Variables|Default|GetIsPlayerControlled)
      (AI|Components|Blackboard|SetValueasBool (AI|GetBlackboard (AI|GetAIController _ascharacter)) (Utilities|Name|MakeLiteralName "IsStunned") false))))