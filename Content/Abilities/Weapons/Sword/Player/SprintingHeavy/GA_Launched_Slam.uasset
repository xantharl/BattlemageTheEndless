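; Gameplay ability for the hit reaction of a character slammed to the ground, filed under the player sword's sprinting heavy attack.
; Plays a montage, then estimates landing time from a downward trace and knockback Z speed to request a stun covering fall plus knockdown.
; On landing, it plays an impact sound, waits that same combined duration, jumps to GetUp, and ends the reaction and ability when the montage ends.
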(event Custom|OnLanded
  (params (Hit :type Hit%20Result%20Structure%20%28by%20ref%29))
  (Audio|PlaySoundatLocation (Variables|Default|GetImpactSound) (stale Ability|EventActivateAbilityFromEvent _pointofimpact) "0, 0, 0" 1.0 1.0 0.25 "/Game/Characters/SoundAttenuation_Default.SoundAttenuation_Default" 0 0 0)
  (Utilities|FlowControl|Delay (+ (stale Ability|EventActivateAbilityFromEvent _timetoland) (Variables|Default|GetPostLandKnockdownTime)))
  (Ability|Animation|MontageJumptoSection (Components|SkeletalMesh|GetAnimInstance (Variables|/Script/Engine.Character|GetMesh (stale Ability|EventActivateAbilityFromEvent _ascharacter))) "GetUp" (Variables|Default|GetMontage%20to%20Play))
  (EventDispatchers|AssignOnMontageEnded (Components|SkeletalMesh|GetAnimInstance (Variables|/Script/Engine.Character|GetMesh (stale Ability|EventActivateAbilityFromEvent _ascharacter))) (delegate Custom|OnMontageEnded_Event)))

(event Custom|OnMontageEnded_Event
  (params (Montage :type Anim%20Montage%20Object%20Reference) (bInterrupted :type Boolean))
  (CallFunction|EndHitReaction (stale Ability|EventActivateAbilityFromEvent _ascharacter))
  (Ability|EndAbility))

(event Ability|EventOnEndAbility
  (params (bWasCancelled :type Boolean)))

(event Ability|EventActivateAbilityFromEvent
  (params (EventData :type Gameplay%20Event%20Data%20Structure%20%28by%20ref%29))
  (bind _ascharacter (Utilities|Casting|CastToCharacter (Ability|GetAvatarActorfromActorInfo))
    (:then
      (Animation|Montage|PlayMontage (Variables|/Script/Engine.Character|GetMesh _ascharacter) (Variables|Default|GetMontage%20to%20Play)
        (:then
          (bind (_timetoland _pointofimpact) (CallFunction|GetTimetoLand))
          (CallFunction|TrySetStunDuration _ascharacter (+ _timetoland (Variables|Default|GetPostLandKnockdownTime)))
          (EventDispatchers|BindEventtoLandedDelegate _ascharacter (delegate Custom|OnLanded)))))
    (:CastFailed
      (Ability|EndAbility))))

(fn GetTimetoLand
  (bind _returnvalue (Ability|GetAvatarActorfromActorInfo))
  (bind _returnvalue_2 (Transformation|GetActorLocation _returnvalue))
  (bind (_outhit _returnvalue_3) (Collision|LineTraceForObjects _returnvalue_2 (+ _returnvalue_2 "0.000000,0.000000,-9999.000000") (LocalVariables|GetTraceObjectTypes) false 0 "None"))
  (if _returnvalue_3
    (return (/ (.z (- _returnvalue_2 (.impactpoint _outhit))) (Math|Float|Absolute(Float) (.z (Variables|Default|GetKnockBackVelocity)))) (.impactpoint _outhit))
    (else
      (return 0.0 "0, 0, 0"))))