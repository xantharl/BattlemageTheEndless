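; GA_Sword_Heavy_Sprint_2 is a player sword ability, by name the second sprinting heavy attack, built on a parent ability's activate and end logic.
; On activation it switches the avatar Character to Flying so root motion can apply vertical movement.
; On end it stops active movement and picks Walking or Falling from IsMovingOnGround before calling the parent.
; LerpGravity is an empty stub.
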(event Ability|EventActivateAbility
  (|CallParentFunction)
  (bind _ascharacter (Utilities|Casting|CastToCharacter (Ability|GetAvatarActorfromActorInfo)))
  (Pawn|Components|CharacterMovement|SetMovementMode (Variables|/Script/Engine.Character|GetCharacterMovement _ascharacter) "MOVE_Flying" 0) ; Root motion only applies Z axis if character is flying
)

(event Ability|EventOnEndAbility
  (params (bWasCancelled :type Boolean))
  (Variables|Default|SetWas%20Cancelled bWasCancelled)
  (bind _ascharacter (Utilities|Casting|CastToCharacter (Ability|GetAvatarActorfromActorInfo)))
  (Class|NavMovementInterface|StopActiveMovement (Variables|/Script/Engine.Character|GetCharacterMovement _ascharacter))
  (Pawn|Components|CharacterMovement|SetMovementMode (Variables|/Script/Engine.Character|GetCharacterMovement _ascharacter) (select (AI|Components|NavMovement|IsMovingonGround (Variables|/Script/Engine.Character|GetCharacterMovement _ascharacter)) "MOVE_Walking" "MOVE_Falling") 0)
  (|CallParentFunction (Variables|Default|GetWas%20Cancelled)))

(fn LerpGravity)