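; Player sword plunge ability, a falling attack that either bounces off a hit or lands on a miss.
; Activation multiplies gravity and binds to weapon-hit and movement-mode events.
; A hit jumps the montage to "Hit" and launches the character with Z override; landing while it plays jumps to "Grounded" and locks movement and controller yaw.
; Ability end unbinds both events and restores gravity, input and yaw.
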(event Custom|MovementModeChangedDelegate_Event
  (params (Character :type Character%20Object%20Reference) (PrevMovementMode :type EMovementMode%20Enum :default "MOVE_None") (PreviousCustomMode :type Byte))
  (CallFunction|OnLanded Character PrevMovementMode))

(event Custom|OnWeaponHit
  (params (character :type Character%20Object%20Reference) (Hit :type Hit%20Result%20Structure%20%28by%20ref%29) (attackAnimationName :type String) (attackOwnedTags :type Gameplay%20Tag%20Container%20Structure))
  (CallFunction|HandleWeaponHit))

(event Ability|EventActivateAbility
  (bind _ascharacter (Utilities|Casting|CastToCharacter (Ability|GetOwningActorfromActorInfo))
    (:then
      (bind _output_get (Variables|Default|SetCharacter _ascharacter))
      (Variables|Default|SetCharacter%20Movement (Variables|/Script/Engine.Character|GetCharacterMovement _output_get))
      (Character|AssignMovementModeChangedDelegate _output_get (delegate Custom|MovementModeChangedDelegate_Event)) ; This handles the miss path, the hit path for advancing montage is handled in the AnimNotify
      (bind _asbmage_ability_system_component (Utilities|Casting|CastToBMageAbilitySystemComponent (Ability|GetAbilitySystemComponent _output_get)))
      (bind _output_get_2 (Variables|Default|SetAs%20BMage%20Ability%20System%20Component _asbmage_ability_system_component))
      (EventDispatchers|BindEventtoOnWeaponHit _output_get_2 (delegate Custom|OnWeaponHit))
      (CallFunction|IncreaseGravity)
      (|CallParentFunction))
    (:CastFailed
      (Utilities|String|LogString "Error in Plunge Fetching Character"))))

(event Ability|EventOnEndAbility
  (params (bWasCancelled :type Boolean))
  (bind _character_movement (Variables|Default|GetCharacter%20Movement))
  (|CallParentFunction bWasCancelled)
  (EventDispatchers|UnbindEventfromOnWeaponHit (Variables|Default|GetAs%20BMage%20Ability%20System%20Component) (delegate Custom|OnWeaponHit))
  (Character|UnbindEventfromMovementModeChangedDelegate (Variables|Default|GetCharacter) (delegate Custom|MovementModeChangedDelegate_Event))
  (Utilities|IsValid _character_movement
    (:Is%20Valid
      (Variables|/Script/Engine.CharacterMovementComponent|SetGravityScale _character_movement (Variables|Default|GetOriginalGravityScale))
      (Input|SetIgnoreMoveInput (Game|GetPlayerController (Variables|/Script/Engine.Pawn|GetPlayerState (Variables|Default|GetCharacter))) false)
      (Variables|/Script/Engine.Pawn|SetbUseControllerRotationYaw (Variables|Default|GetCharacter) true))))

(fn OnLanded
  (params (Character :type Character%20Object%20Reference) (PrevMode :type EMovementMode%20Enum :default "MOVE_None"))
  (if (Utilities|Enum|Equal(Enum) (Variables|/Script/Engine.CharacterMovementComponent|GetMovementMode (Variables|Default|GetCharacter%20Movement)) "MOVE_Walking")
    (if (Class|AnimInstance|DynamicMontageIsPlayingfrom (Components|SkeletalMesh|GetAnimInstance (Variables|/Script/Engine.Character|GetMesh Character)) (Variables|Default|GetFireAnimation))
      (Ability|Animation|MontageJumptoSection "Grounded")
      (Input|SetIgnoreMoveInput (Game|GetPlayerController (Variables|/Script/Engine.Pawn|GetPlayerState Character)) true)
      (Variables|/Script/Engine.Pawn|SetbUseControllerRotationYaw (Variables|Default|GetCharacter) false)
      (return))
    (else
      (return))))

(fn IncreaseGravity
  (bind _output_get (Variables|Default|SetOriginalGravityScale (Variables|/Script/Engine.CharacterMovementComponent|GetGravityScale (Variables|Default|GetCharacter%20Movement))))
  (Variables|/Script/Engine.CharacterMovementComponent|SetGravityScale (Variables|Default|GetCharacter%20Movement) (* _output_get (Variables|Default|GetGravityScaleMultiplier))))

(fn HandleWeaponHit
  (Ability|Animation|MontageJumptoSection "Hit")
  (Character|LaunchCharacter (Variables|Default|GetCharacter) (Variables|Default|GetBounceLaunchVector) false true))