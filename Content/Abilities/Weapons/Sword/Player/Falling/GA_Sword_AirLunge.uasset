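; Player sword gameplay ability for a lunge while airborne, aimed along the camera's pitch.
; On activation it runs the parent logic, switches the character to Flying so root motion applies on Z, enables controller pitch rotation and pitches the root by the camera's pitch.
; On end it disables controller pitch and sets movement to Walking or Falling based on an on-ground check.
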(event Ability|EventActivateAbility
  (|CallParentFunction)
  (bind _ascharacter (Utilities|Casting|CastToCharacter (Ability|GetAvatarActorfromActorInfo)))
  (bind _output_get (Variables|Default|SetOwningCharacter _ascharacter))
  (Pawn|Components|CharacterMovement|SetMovementMode (Variables|/Script/Engine.Character|GetCharacterMovement _output_get) "MOVE_Flying" 0) ; Root motion only applies Z axis if character is flying
  (Variables|/Script/Engine.Pawn|SetbUseControllerRotationPitch _output_get true)
  (Transformation|AddWorldRotation (Variables|/Script/Engine.Actor|GetRootComponent _output_get) (Math|Rotator|MakeRotator 0.0 (.pitch (Camera|GetCameraRotation (Variables|/Script/Engine.PlayerController|GetPlayerCameraManager (Game|GetPlayerController 0)))) 0.0) false false))

(event Ability|EventOnEndAbility
  (params (bWasCancelled :type Boolean))
  (|CallParentFunction bWasCancelled)
  (Pawn|Components|CharacterMovement|SetMovementMode (Variables|/Script/Engine.Character|GetCharacterMovement (stale Ability|EventActivateAbility _output_get)) (select (AI|Components|NavMovement|IsMovingonGround (Variables|/Script/Engine.Character|GetCharacterMovement (stale Ability|EventActivateAbility _output_get))) "MOVE_Walking" "MOVE_Falling") 0) ; Root motion only applies Z axis if character is flying
  (Variables|/Script/Engine.Pawn|SetbUseControllerRotationPitch (Variables|Default|GetOwningCharacter) false))