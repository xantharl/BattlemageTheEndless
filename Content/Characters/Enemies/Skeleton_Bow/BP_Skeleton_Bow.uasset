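; BP_Skeleton_Bow is a skeleton enemy character blueprint, named as the bow variant, assembled from several skeletal mesh parts.
; Its construction script runs the parent's script, then sets the main Mesh as leader pose component for the extra skeletal meshes so they share one pose.
; The event graph holds only a disabled overlap placeholder, so this blueprint adds no gameplay logic in its graphs.
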(event Collision|EventActorBeginOverlap
  (params (OtherActor :type Actor%20Object%20Reference)))

(fn ConstructionScript
  (|CallParentFunction)
  (Components|SkinnedMesh|SetLeaderPoseComponent (Variables|Default|GetSkeletalMesh7) (Variables|Character|GetMesh) false false))