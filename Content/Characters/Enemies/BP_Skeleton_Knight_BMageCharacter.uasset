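; Skeleton Knight BMage enemy character, built from modular skeletal meshes that follow the main mesh through Leader Pose, set in the construction script.
; On BeginPlay it writes its current attack range to the Blackboard.
; JumptoDestination computes an arc velocity to a point raised above the target by root bounds and an offset, prints it, and launches the character with it, overriding existing velocity.
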(event EventJumptoDestination
  (params (Destination :type Vector :default "0, 0, 0"))
  (bind _outlaunchvelocity (Game|SuggestProjectileVelocityCustomArc (Transformation|GetActorLocation) (Math|Vector|MakeVector (.x Destination) (.y Destination) (+ (+ (.z Destination) (.z (.BoxExtent (Collision|GetComponentBounds (Variables|Transformation|GetRootComponent))))) 1e+02)) 0.0 0.5))
  (Development|PrintString (Utilities|String|ToString(Vector) _outlaunchvelocity))
  (Character|LaunchCharacter _outlaunchvelocity true true))

(event Collision|EventActorBeginOverlap
  (params (OtherActor :type Actor%20Object%20Reference)))

(event EventTick
  (params (DeltaSeconds :type Float%20%28single-precision%29))
  (|CallParentFunction DeltaSeconds) ; This node is disabled and will not be called.\nDrag off pins to build functionality.
)

(event EventBeginPlay
  (AI|Components|Blackboard|SetValueasFloat (AI|GetBlackboard 0) (Utilities|Name|MakeLiteralName "CurrentAttackRange") 1e+02))

(fn ConstructionScript
  (|CallParentFunction)
  (Components|SkinnedMesh|SetLeaderPoseComponent (Variables|Default|GetSkeletalMesh7) (Variables|Character|GetMesh) false false))