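; Stationary training dummy character that reacts physically when struck by melee weapons.
; On BeginPlay it binds to the ability system component's weapon-hit event, which AnimTrace fires.
; Each hit briefly enables physical animation and passes the hit and attacker to the physical animation component for a reaction, then disables it after a short delay.
; Tick rotates the health bar widget to face the player camera.
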(event Custom|OnWeaponHit_Event
  (params (character :type Character%20Object%20Reference) (Hit :type Hit%20Result%20Structure%20%28by%20ref%29) (attackAnimationName :type String))
  (bind _physanimcomp (Variables|Default|GetPhysAnimComp))
  (Default|TogglePhysicalAnimation _physanimcomp true)
  (Default|HitReaction _physanimcomp Hit character)
  (Utilities|FlowControl|Delay 0.5)
  (Default|TogglePhysicalAnimation _physanimcomp false))

(event EventBeginPlay
  (|CallParentFunction)
  (EventDispatchers|AssignOnWeaponHit (Variables|Default|GetAbilitySystemComponent) (delegate Custom|OnWeaponHit_Event)) ; Fired by AnimTrace for melee
)

(event EventTick
  (params (DeltaSeconds :type Float%20%28single-precision%29))
  (bind _health_bar_widget_component (Variables|Default|GetHealth%20Bar%20Widget%20Component))
  (Transformation|SetWorldRotation _health_bar_widget_component (Math|Rotator|FindLookatRotation (Transformation|GetWorldLocation _health_bar_widget_component) (Transformation|GetWorldLocation (Variables|/Script/Engine.PlayerCameraManager|GetTransformComponent (Game|GetPlayerCameraManager 0)))) false false))

(fn ConstructionScript)