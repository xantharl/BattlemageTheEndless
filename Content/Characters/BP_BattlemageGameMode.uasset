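; BP_BattlemageGameMode is a game mode Blueprint that handles player restarts and applies loaded save data.
; On restart, it passes the player controller to the SwarmManager.
; LoadGameState copies saved character creation data into the BMageGameInstance, destroys the indexed player's pawn, then respawns that player at the saved transform.
; It receives the save data already loaded and leaves its SlotName input unused.
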(event EventOnRestartPlayer
  (params (NewPlayer :type Controller%20Object%20Reference))
  (bind _asplayer_controller (Utilities|Casting|CastToPlayerController NewPlayer))
  (Class|SwarmManagerComponent|RestartPlayer (Variables|Default|GetSwarmManager) _asplayer_controller))

(fn ConstructionScript)

(fn LoadGameState
  (params (SlotName :type String) (UserIndex :type Integer) (LoadedGameData :type B%20Mage%20Local%20Player%20Save%20Game%20Object%20Reference))
  (bind _returnvalue (Game|GetPlayerController UserIndex))
  (bind _asbmage_game_instance (Utilities|Casting|CastToBMageGameInstance (Game|GetGameInstance)))
  (Variables|/Game/Maps/BMageGameInstance.BMageGameInstance_C|SetCharacterCreationData _asbmage_game_instance (Variables|/Script/BattlemageTheEndless.BMageLocalPlayerSaveGame|GetCharacterCreationData LoadedGameData))
  (Actor|DestroyActor (Pawn|GetControlledPawn _returnvalue))
  (Class|GameModeBase|RestartPlayeratTransform _returnvalue (Variables|/Script/BattlemageTheEndless.BMageLocalPlayerSaveGame|GetPlayerTransform LoadedGameData)))