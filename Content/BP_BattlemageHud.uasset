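; Battlemage HUD that creates the W_BMageHud widget for the owning player and registers itself on BP_BattlemageCharacter.
; On BeginPlay it builds the widget at once if a pawn is possessed, otherwise it waits for OnPossessedPawnChanged.
; MenuOpened, fired by the character, and MenuClosed toggle the top and bottom menus, mouse cursor and UI-only or game-only input mode.
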(event Custom|OnPossessedPawnChanged_Event
  (params (OldPawn :type Pawn%20Object%20Reference) (NewPawn :type Pawn%20Object%20Reference))
  (Utilities|IsValid NewPawn
    (:Is%20Valid
      (bind _returnvalue (UserInterface|CreateWidget "/Game/fantasy_gui_4/widgets/W_BMageHud.W_BMageHud_C" (stale EventBeginPlay _output_get)))
      (bind _output_get (Variables|Default|SetHudWidget _returnvalue))
      (UserInterface|Viewport|AddtoViewport _output_get 0)
      (bind _asbp_battlemage_character (Utilities|Casting|CastToBP_BattlemageCharacter (Class|HUD|GetOwningPawn)))
      (Variables|/Game/Characters/BP_BattlemageCharacter.BP_BattlemageCharacter_C|SetHUD _asbp_battlemage_character self))))

(event EventBeginPlay
  (bind _output_get (Variables|Default|SetPlayerController (Game|Player|GetOwningPlayerController)))
  (Utilities|IsValid (Pawn|GetControlledPawn _output_get)
    (:Is%20Valid
      (bind _returnvalue (UserInterface|CreateWidget "/Game/fantasy_gui_4/widgets/W_BMageHud.W_BMageHud_C" _output_get))
      (bind _output_get_2 (Variables|Default|SetHudWidget _returnvalue))
      (UserInterface|Viewport|AddtoViewport _output_get_2 0)
      (bind _asbp_battlemage_character (Utilities|Casting|CastToBP_BattlemageCharacter (Class|HUD|GetOwningPawn)))
      (Variables|/Game/Characters/BP_BattlemageCharacter.BP_BattlemageCharacter_C|SetHUD _asbp_battlemage_character self))
    (:Is%20Not%20Valid
      (EventDispatchers|AssignOnPossessedPawnChanged _output_get (delegate Custom|OnPossessedPawnChanged_Event)))))

(event Collision|EventActorBeginOverlap
  (params (OtherActor :type Actor%20Object%20Reference)))

(event EventTick
  (params (DeltaSeconds :type Float%20%28single-precision%29)))

(event EventMenuOpened
  (bind _hudwidget (Variables|Default|GetHudWidget))
  (bind _playercontroller (Variables|Default|GetPlayerController))
  (bind _hudwidget_2 (Variables|Default|GetHudWidget))
  (bind _w_window_gameview (Variables|/Game/fantasy_gui_4/widgets/W_BMageHud.W_BMageHud_C|GetW_Window_GameView _hudwidget_2))
  ;[1 1 1 1 14] Event Fires by BP_BattlemageCharacter when the appropriate IA is triggered
  (Widget|SetVisibility (Variables|/Game/fantasy_gui_4/widgets/sample_windows/W_Window_GameView.W_Window_GameView_C|GetW_TopMenu _w_window_gameview) "Visible")
  (Widget|SetVisibility (Variables|/Game/fantasy_gui_4/widgets/sample_windows/W_Window_GameView.W_Window_GameView_C|GetW_BottomMenu _w_window_gameview) "Visible")
  (Input|SetInputModeUIOnly _playercontroller _hudwidget "LockAlways" false)
  (Variables|/Script/Engine.PlayerController|SetbShowMouseCursor _playercontroller true)
  (Widget|SetKeyboardFocus _hudwidget))

(event EventMenuClosed
  (bind _playercontroller (Variables|Default|GetPlayerController))
  (bind _hudwidget (Variables|Default|GetHudWidget))
  (bind _w_window_gameview (Variables|/Game/fantasy_gui_4/widgets/W_BMageHud.W_BMageHud_C|GetW_Window_GameView _hudwidget))
  ;[1 1 1 1 12] Listening for specific keys since I don't know how to use input actions in UI only mode
  (Widget|SetVisibility (Variables|/Game/fantasy_gui_4/widgets/sample_windows/W_Window_GameView.W_Window_GameView_C|GetW_TopMenu _w_window_gameview) "Hidden")
  (Widget|SetVisibility (Variables|/Game/fantasy_gui_4/widgets/sample_windows/W_Window_GameView.W_Window_GameView_C|GetW_BottomMenu _w_window_gameview) "Hidden")
  (Input|SetInputModeGameOnly _playercontroller false)
  (Variables|/Script/Engine.PlayerController|SetbShowMouseCursor _playercontroller false))

(fn ConstructionScript)