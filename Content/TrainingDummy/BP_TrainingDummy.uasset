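; Training dummy actor with an Ability System Component and a world-space health bar widget.
; On Tick it rotates the health bar component to face the player camera.
; A disconnected, deprecated chain once filled the bar from BaseAttributeSet health and showed FireBolt DoT stacks; its comment says that logic moved to the UHealthBarWidget C++ class.
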(event EventTick
  (params (DeltaSeconds :type Float%20%28single-precision%29))
  (bind _health_bar_widget_component (Variables|Default|GetHealth%20Bar%20Widget%20Component))
  (Transformation|SetWorldRotation _health_bar_widget_component (Math|Rotator|FindLookatRotation (Transformation|GetWorldLocation _health_bar_widget_component) (Transformation|GetWorldLocation (Variables|/Script/Engine.PlayerCameraManager|GetTransformComponent (Game|GetPlayerCameraManager 0)))) false false))

(fn ConstructionScript)