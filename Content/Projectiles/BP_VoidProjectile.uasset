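; BP_VoidProjectile is a projectile actor whose graph handles only its visual effects.
; On BeginPlay it spawns a muzzle burst at the Sphere component's transform and assigns the projectile effect to its Muzzle Niagara component.
; When destroyed, it spawns a scaled-down hit effect at the sphere's location, so the effect follows any destruction rather than a specific hit event.
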(event EventBeginPlay
  (bind _sphere (Variables|Default|GetSphere))
  (Niagara|SpawnSystematLocation (Variables|Default|GetMuzzle%20FX) (Transformation|GetWorldLocation _sphere) (Transformation|GetWorldRotation _sphere))
  (Class|NiagaraComponent|SetAsset (Variables|Default|GetMuzzle) (Variables|Default|GetProjectile%20FX) true))

(event EventDestroyed
  (Niagara|SpawnSystematLocation (Variables|Default|GetHit%20FX) (Transformation|GetWorldLocation (Variables|Default|GetSphere)) "0, 0, 0" "0.250000,0.250000,0.250000"))

(fn ConstructionScript)